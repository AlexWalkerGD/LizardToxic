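; Ground_Child1 is a child Blueprint of a ground actor that acts as a lethal hazard for the Lizard character.
; When a Lizard overlaps its box, the Blueprint zeroes its walk speed, hides its mesh and flags it dead.
; It then shows the Restart widget, pauses the game and switches to UI-only input with a visible cursor.
; The construction script only calls the parent's.
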(event OnComponentBeginOverlap(Box_0)
  (params (OverlappedComponent :type Primitive%20Component%20Object%20Reference) (OtherActor :type Actor%20Object%20Reference) (OtherComp :type Primitive%20Component%20Object%20Reference) (OtherBodyIndex :type Integer) (bFromSweep :type Boolean) (SweepResult :type Hit%20Result%20Structure%20%28by%20ref%29))
  (bind _returnvalue (Game|GetPlayerController 0))
  (bind _aslizard (Utilities|Casting|CastToLizard OtherActor))
  (Variables|/Script/Engine.CharacterMovementComponent|SetMaxWalkSpeed (Variables|/Script/Engine.Character|GetCharacterMovement _aslizard) 0.0)
  (Rendering|SetVisibility (Variables|/Script/Engine.Character|GetMesh _aslizard) false false)
  (Variables|/Game/Lizard/Blueprints/System/Lizard.Lizard_C|SetIsDead _aslizard true)
  (bind _returnvalue_2 (UserInterface|CreateWidget "/Game/Lizard/UI/Restart.Restart_C"))
  (UserInterface|Viewport|AddtoViewport _returnvalue_2 0)
  (Game|SetGamePaused true)
  (Input|SetInputModeUIOnly _returnvalue _returnvalue_2 "DoNotLock")
  (Variables|/Script/Engine.PlayerController|SetbShowMouseCursor _returnvalue true))

(fn ConstructionScript
  (|CallParentFunction))